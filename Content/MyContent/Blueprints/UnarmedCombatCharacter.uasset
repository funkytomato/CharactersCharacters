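; Character Blueprint for unarmed combat that turns player input into punch, kick, block and evasion state.
; Each input action sets a matching boolean while held and clears it on release, covering left and right jabs, hooks, uppercuts, low kicks, dodges and ducks.
; The file only tracks these flags; it contains no animation, damage or movement logic, and the construction script just calls its parent.
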(event Input|ActionEvents|InputActionLeftJab
  (params (Key :type Key%20Structure :default "None"))
  (:Pressed
    (Variables|Default|SetIsLeftJab true))
  (:Released
    (Variables|Default|SetIsLeftJab false)))

(event Input|ActionEvents|InputActionRightJab
  (params (Key :type Key%20Structure :default "None"))
  (:Pressed
    (Variables|Default|SetIsRightJab true))
  (:Released
    (Variables|Default|SetIsRightJab false)))

(event Input|ActionEvents|InputActionDuckLeft
  (params (Key :type Key%20Structure :default "None"))
  (:Pressed
    (Variables|Default|SetIsDuckingLeft true))
  (:Released
    (Variables|Default|SetIsDuckingLeft false)))

(event Input|ActionEvents|InputActionDuckRight
  (params (Key :type Key%20Structure :default "None"))
  (:Pressed
    (Variables|Default|SetIsDuckingRight true))
  (:Released
    (Variables|Default|SetIsDuckingRight false)))

(event Input|ActionEvents|InputActionLeftLowKick
  (params (Key :type Key%20Structure :default "None"))
  (:Pressed
    (Variables|Default|SetIsLeftLowKick true))
  (:Released
    (Variables|Default|SetIsLeftLowKick false)))

(event Input|ActionEvents|InputActionRightLowKick
  (params (Key :type Key%20Structure :default "None"))
  (:Pressed
    (Variables|Default|SetIsRightLowKick true))
  (:Released
    (Variables|Default|SetIsRightLowKick false)))

(event Input|ActionEvents|InputActionLeftHook
  (params (Key :type Key%20Structure :default "None"))
  (:Pressed
    (Variables|Default|SetIsLeftHook true))
  (:Released
    (Variables|Default|SetIsLeftHook false)))

(event Input|ActionEvents|InputActionRightHook
  (params (Key :type Key%20Structure :default "None"))
  (:Pressed
    (Variables|Default|SetIsRightHook true))
  (:Released
    (Variables|Default|SetIsRightHook false)))

(event Input|ActionEvents|InputActionBlock
  (params (Key :type Key%20Structure :default "None"))
  (:Pressed
    (Variables|Default|SetIsBlocking true))
  (:Released
    (Variables|Default|SetIsBlocking false)))

(event Input|ActionEvents|InputActionLeftUpperCut
  (params (Key :type Key%20Structure :default "None"))
  (:Pressed
    (Variables|Default|SetIsLeftUpperCut true))
  (:Released
    (Variables|Default|SetIsLeftUpperCut false)))

(event Input|ActionEvents|InputActionRightUpperCut
  (params (Key :type Key%20Structure :default "None"))
  (:Pressed
    (Variables|Default|SetIsRightUpperCut true))
  (:Released
    (Variables|Default|SetIsRightUpperCut false)))

(event Input|ActionEvents|InputActionDodgeLeft
  (params (Key :type Key%20Structure :default "None"))
  (:Pressed
    (Variables|Default|SetIsDodgeLeft true))
  (:Released
    (Variables|Default|SetIsDodgeLeft false)))

(event Input|ActionEvents|InputActionDodgeRight
  (params (Key :type Key%20Structure :default "None"))
  (:Pressed
    (Variables|Default|SetIsDodgeRight true))
  (:Released
    (Variables|Default|SetIsDodgeRight false)))

(event Input|ActionEvents|InputActionDuck
  (params (Key :type Key%20Structure :default "None"))
  (:Pressed
    (Variables|Default|SetIsDucking true))
  (:Released
    (Variables|Default|SetIsDucking false)))

(fn ConstructionScript
  (|CallParentFunction))